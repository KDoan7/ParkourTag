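; Grappling hook projectile that flies out from its spawn point and destroys itself once it travels too far.
; BeginPlay feeds a Velocity variable into the ProjectileMovement component and records the start location, which Tick checks against MaxDistance.
; When it overlaps its owner, it waits briefly, then sets the mesh to block the Pawn channel.
; The mesh hit event is empty, so no attach or pull logic exists here.
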(event `self.ReceiveBeginPlay`
  (set `MovementComponent.Velocity` (`self.Velocity`) (`self.ProjectileMovement`))
  (set `self.Start Location` (`self.K2_GetActorLocation`)))

(event `self.ReceiveActorBeginOverlap`
  (params (OtherActor :type "Actor Object Reference"))
  (if (not (!= OtherActor (`self.GetOwner`)))
    (`KismetSystemLibrary.Delay` 0.01)
    (`PrimitiveComponent.SetCollisionResponseToChannel` (`self.StaticMesh`) "ECC_Pawn" "ECR_Block")))

(event `self.ReceiveTick`
  (params (DeltaSeconds :type "Float (single-precision)"))
  (if (>= (`KismetMathLibrary.Vector_Distance` (`self.Start Location`) (`self.K2_GetActorLocation`)) (`self.MaxDistance`))
    (`self.K2_DestroyActor`)))

(event `self.StaticMesh.OnComponentHit`
  (params (HitComponent :type "PrimitiveComponent Object Reference") (OtherActor :type "Actor Object Reference") (OtherComp :type "PrimitiveComponent Object Reference") (NormalImpulse :type "Vector Structure") (Hit :type "HitResult Structure (by ref)")))

(fn `UserConstructionScript`)