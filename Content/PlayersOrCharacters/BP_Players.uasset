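; Player character Blueprint with a grappling hook, pause menu input and a camera spring arm attached to the mesh's head socket.
; Grapple input traces from the camera to pick a target for GrapplingComponent, or cancels an active grapple.
; Capsule hits cancel the grapple in one state when no player is hooked.
; A cooldown flag gates firing, but its delayed reset is unconnected here.
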(event `InputAction|GrapplingHook`
  (params (Key :type "Key Structure"))
  (bind _returnvalue (`SceneComponent.K2_GetComponentLocation` (`self.Camera`)))
  (:`Pressed`
    (if (`self.Grapple Cooldown Reached`)
      (if (`/Game/GrapplingHook/GrapplingComponent.IsInUse` (`self.GrapplingComponent`))
        (`/Game/GrapplingHook/GrapplingComponent.CancelGrapple` (`self.GrapplingComponent`))
        (else
          (set `self.Grapple Cooldown Reached` false)
          (bind (_outhit _returnvalue_2) (`KismetSystemLibrary.LineTraceSingle` _returnvalue (+ _returnvalue (* (`SceneComponent.GetForwardVector` (`self.Camera`)) 15000.0)) "TraceTypeQuery1"))
          (bind (_bblockinghit _binitialoverlap _time _distance _location _impactpoint _normal _impactnormal _physmat _hitactor _hitcomponent _hitbonename _bonename _hititem _elementindex _faceindex _tracestart _traceend) (`GameplayStatics.BreakHitResult` _outhit))
          (`/Game/GrapplingHook/GrapplingComponent.FireGrapplingHook` (`self.GrapplingComponent`) (select `bool` _returnvalue_2 :`false` _traceend :`true` _location) (0.0 0.0 50.0))))
      (else
        (`/Game/GrapplingHook/GrapplingComponent.CancelGrapple` (`self.GrapplingComponent`))))))

(event `GrapplingHookCoolDown`)

(event `self.ReceiveBeginPlay`)

(event `self.ReceiveTick`
  (params (DeltaSeconds :type "Float (single-precision)")))

(event `self.ReceiveActorBeginOverlap`
  (params (OtherActor :type "Actor Object Reference")))

(event `self.CapsuleComponent.OnComponentHit`
  (params (HitComponent :type "PrimitiveComponent Object Reference") (OtherActor :type "Actor Object Reference") (OtherComp :type "PrimitiveComponent Object Reference") (NormalImpulse :type "Vector Structure") (Hit :type "HitResult Structure (by ref)"))
  (if (and (`|EnumEquality` (`/Game/GrapplingHook/GrapplingComponent.GrappleState` (`self.GrapplingComponent`)) "NewEnumerator2") (not (`KismetSystemLibrary.IsValid` (`/Game/GrapplingHook/GrapplingComponent.PlayerHit` (`self.GrapplingComponent`)))))
    (`/Game/GrapplingHook/GrapplingComponent.CancelGrapple` (`self.GrapplingComponent`))))

(event `InputAction|PauseMenu`
  (params (Key :type "Key Structure"))
  (:`Pressed`
    (bind _returnvalue (`|CreateWidget` "/Game/Levels/MainMenu/MainMenu.MainMenu_C"))
    (`UserWidget.AddToViewport` _returnvalue 0)
    (set `PlayerController.bShowMouseCursor` true (`GameplayStatics.GetPlayerController` 0))
    (`WidgetBlueprintLibrary.SetInputMode_UIOnlyEx` (`GameplayStatics.GetPlayerController` 0) null)))

(fn `UserConstructionScript`
  (`SceneComponent.K2_AttachToComponent` (`self.SpringArmComp`) (`self.Mesh`) "head" "KeepRelative" "KeepRelative" "KeepRelative" true)
  (`SceneComponent.K2_SetWorldTransform` (`self.SpringArmComp`) (`KismetMathLibrary.Conv_VectorToTransform` (+ (`SceneComponent.GetSocketLocation` (`self.Mesh`) "head") (0.0 0.0 0.0))) false false))