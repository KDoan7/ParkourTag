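; Player character with a grappling hook, a head-mounted camera arm and a HUD.
; Grapple input traces from the camera and fires GrapplingComponent at the hit or trace end, or cancels an active grapple; a delayed event restores the cooldown flag.
; Capsule hits cancel the grapple in one state when no player is hooked.
; Tick prints movement, speed, wall-run, wall-climb and grapple-readiness debug values.
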(event `InputAction|GrapplingHook`
  (params (Key :type "Key Structure"))
  (bind _returnvalue (`SceneComponent.K2_GetComponentLocation` (`self.Camera`)))
  (:`Pressed`
    (if (`self.Grapple Cooldown Reached`)
      (if (`/Game/GrapplingHook/GrapplingComponent.IsInUse` (`self.GrapplingComponent`))
        (`/Game/GrapplingHook/GrapplingComponent.CancelGrapple` (`self.GrapplingComponent`))
        (else
          (set `self.Grapple Cooldown Reached` false)
          (bind (_outhit _returnvalue_2) (`KismetSystemLibrary.LineTraceSingle` _returnvalue (+ _returnvalue (* (`SceneComponent.GetForwardVector` (`self.Camera`)) 15000.0)) "TraceTypeQuery1"))
          (bind (_bblockinghit _binitialoverlap _time _distance _location _impactpoint _normal _impactnormal _physmat _hitactor _hitcomponent _hitbonename _bonename _hititem _elementindex _faceindex _tracestart _traceend) (`GameplayStatics.BreakHitResult` _outhit))
          (`/Game/GrapplingHook/GrapplingComponent.FireGrapplingHook` (`self.GrapplingComponent`) (select `bool` _returnvalue_2 :`false` _traceend :`true` _location) (0.0 0.0 10.0))))
      (else
        (`/Game/GrapplingHook/GrapplingComponent.CancelGrapple` (`self.GrapplingComponent`))))))

(event `GrapplingHookCoolDown`
  (`KismetSystemLibrary.Delay` (`self.Cool Down Timer`))
  (set `self.Grapple Cooldown Reached` true))

(event `self.ReceiveBeginPlay`
  (bind _returnvalue (`|CreateWidget` "/Game/HUD/HUD2.HUD2_C"))
  (`UserWidget.AddToViewport` _returnvalue 0))

(event `self.ReceiveActorBeginOverlap`
  (params (OtherActor :type "Actor Object Reference")))

(event `self.ReceiveTick`
  (params (DeltaSeconds :type "Float (single-precision)"))
  (`KismetSystemLibrary.PrintString` (`KismetStringLibrary.JoinStringArray` (`|MakeArray` (`self.CurrentMoveStateString`) (`|GetEnumeratorNameAsString` (`self.currentMovementState`)))) true true (struct :`R` 1.0 :`G` 0.84455 :`A` 1.0) 1.0 "0")
  (`KismetSystemLibrary.PrintString` (`KismetStringLibrary.JoinStringArray` (`|MakeArray` (`self.Current Speed String`) (`KismetStringLibrary.Conv_DoubleToString` (`KismetMathLibrary.VSize` (`MovementComponent.Velocity` (`self.CharacterMovement`)))))) true true (struct :`R` 1.0 :`G` 0.067573 :`B` 0.418076 :`A` 1.0) 1.0 "1")
  (`KismetSystemLibrary.PrintString` (`KismetStringLibrary.JoinStringArray` (`|MakeArray` (`self.Wall Climb Speed String`) (`KismetStringLibrary.Conv_DoubleToString` (`self.wallClimbHeight`)))) true true (struct :`G` 0.66 :`B` 1.0 :`A` 1.0) 1.0 "2")
  (`KismetSystemLibrary.PrintString` (`KismetStringLibrary.JoinStringArray` (`|MakeArray` (`self.Is Wall Running String`) (`KismetStringLibrary.Conv_BoolToString` (`self.isWallRunning`)))) true true (struct :`R` 0.336666 :`G` 1.0 :`B` 0.033717 :`A` 1.0) 1.0 "3")
  (`KismetSystemLibrary.PrintString` (`KismetStringLibrary.JoinStringArray` (`|MakeArray` (`self.is Wall Climbing String`) (`KismetStringLibrary.Conv_BoolToString` (`self.isWallClimbing`)))) true true (struct :`R` 0.622236 :`G` 0.031798 :`B` 1.0 :`A` 1.0) 1.0 "4")
  (`KismetSystemLibrary.PrintString` (`KismetStringLibrary.JoinStringArray` (`|MakeArray` (`self.CanGrapple`) (`KismetStringLibrary.Conv_BoolToString` (`self.Grapple Cooldown Reached`)))) true true (struct :`R` 1.0 :`G` 0.540051 :`A` 1.0) 1.0 "5"))

(event `self.CapsuleComponent.OnComponentHit`
  (params (HitComponent :type "PrimitiveComponent Object Reference") (OtherActor :type "Actor Object Reference") (OtherComp :type "PrimitiveComponent Object Reference") (NormalImpulse :type "Vector Structure") (Hit :type "HitResult Structure (by ref)"))
  (if (and (`|EnumEquality` (`/Game/GrapplingHook/GrapplingComponent.GrappleState` (`self.GrapplingComponent`)) "NewEnumerator2") (not (`KismetSystemLibrary.IsValid` (`/Game/GrapplingHook/GrapplingComponent.PlayerHit` (`self.GrapplingComponent`)))))
    (`/Game/GrapplingHook/GrapplingComponent.CancelGrapple` (`self.GrapplingComponent`))))

(fn `UserConstructionScript`
  (`SceneComponent.K2_AttachToComponent` (`self.SpringArmComp`) (`self.Mesh`) "head" "KeepRelative" "KeepRelative" "KeepRelative" true)
  (`SceneComponent.K2_SetWorldTransform` (`self.SpringArmComp`) (`KismetMathLibrary.Conv_VectorToTransform` (+ (`SceneComponent.GetSocketLocation` (`self.Mesh`) "head") (0.0 0.0 0.0))) false false))