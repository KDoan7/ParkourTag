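; Game mode that assigns player starts and spawns grappling hook pickups.
; ChoosePlayerStart scans NonItPlayerSpawn actors and tags the first untaken one as "Taken" to reserve it.
; SpawnHookPickup waits through a short delay, then spawns a GrapplingHookPickup at a stored location.
; The construction script fills RandomSpawnSpots with hardcoded transforms, which nothing in this graph reads.
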(event `self.ReceiveBeginPlay`)

(event `SpawnHookPickup`
  (`KismetSystemLibrary.Delay` 5.0)
  (`|SpawnActorFromClass` "/Game/PickUps/GrapplingHookPickup.GrapplingHookPickup_C" (`KismetMathLibrary.MakeTransform` (`self.Spawn GrappleHook Pickup Location`)) "Undefined" "OverrideRootScale" null null))

(fn `ChoosePlayerStart`
  (params (Player :type "Controller Object Reference"))
  (returns (ReturnValue :type "Actor Object Reference"))
  (bind _outactors (`GameplayStatics.GetAllActorsOfClass` "/Game/PlayerSpawn/NonItPlayerSpawn.NonItPlayerSpawn_C"))
  (for _array_element _outactors
    (if (!= (`PlayerStart.PlayerStartTag` _array_element) "Taken")
      (set `PlayerStart.PlayerStartTag` "Taken" _array_element)
      (return null))))

(fn `UserConstructionScript`
  (set `self.Random Spawn spots` (`|MakeArray` (`KismetMathLibrary.MakeTransform` (-4730.0 -310.0 602.0)) (`KismetMathLibrary.MakeTransform` (-4730.0 220.0 602.0)) (`KismetMathLibrary.MakeTransform` (-4730.0 750.0 602.0)))))